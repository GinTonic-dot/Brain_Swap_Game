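; Collectable world item that the player picks up through interaction and carries, one at a time.
; Interact stores it as the player's HeldCollectable if none is held, disables mesh collision and shadows, snaps it to CollectablePivot a tick later, then fires the collected dispatcher.
; PlaceCollectable restores shadows and sets mesh visibility and collision, without detaching it itself.
; An interactable flag is exposed through setter and getter functions.
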(event Custom|PlaceCollectable
  (Rendering|SetCastShadow (Variables|Default|GetMesh) true)
  (Collision|SetCollisionEnabled (Variables|Default|GetMesh) "QueryAndPhysics")
  (Rendering|SetVisibility (Variables|Default|GetMesh) (Variables|Default|GetbNewVisibility) false)
  (Variables|Default|GetbNewVisibility
    (:then)
    (:else
      (Collision|SetCollisionEnabled (Variables|Default|GetMesh) "NoCollision"))))

(event EventInteract
  (params (Sender :type Actor%20Object%20Reference))
  (bind _asbp_player (Utilities|Casting|CastToBP_Player Sender))
  (Variables|/Game/Blueprints/Core/BP_Player.BP_Player_C|GetHeldCollectable _asbp_player
    (:then)
    (:else
      (Variables|/Game/Blueprints/Core/BP_Player.BP_Player_C|SetHeldCollectable _asbp_player self)
      (Collision|SetCollisionEnabled (Variables|Default|GetMesh) "NoCollision")
      (Utilities|FlowControl|DelayUntilNextTick)
      (Transformation|AttachComponentToComponent (Variables|/Game/Blueprints/Core/BP_Player.BP_Player_C|GetCollectablePivot _asbp_player) "None" "SnapToTarget" "SnapToTarget" "SnapToTarget" true)
      (Rendering|SetCastShadow (Variables|Default|GetMesh) false)
      (Collision|SetCollisionEnabled (Variables|Default|GetMesh) "NoCollision")
      (Default|CallOnCollectedDispatcher))))

(event EventSetInteractStatus
  (params (IsInteractable :type Boolean))
  (Variables|Default|SetIs%20Interactable IsInteractable))

(fn ConstructionScript)

(fn ReturnInteractStatus
  (return (Variables|Default|GetIs%20Interactable)))