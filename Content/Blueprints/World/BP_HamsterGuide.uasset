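; Hamster guide NPC that turns toward the player and shows tutorial dialog lines.
; Speech starts on interaction or an optional, optionally one-shot, overlap trigger, both playing a scale wobble timeline.
; GetNextDialogLine steps through DialogLines, then loops or holds the last line, returning a fallback line when the list is empty or play-once dialog is used up.
; SpeakToPlayer passes the line to BP_Player's tutorial display.
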(event OnComponentBeginOverlap(AutoTriggerCollision)
  (params (OverlappedComponent :type Primitive%20Component%20Object%20Reference) (OtherActor :type Actor%20Object%20Reference) (OtherComp :type Primitive%20Component%20Object%20Reference) (OtherBodyIndex :type Integer) (bFromSweep :type Boolean) (SweepResult :type Hit%20Result%20Structure%20%28by%20ref%29))
  (if (Variables|Default|GetbAutoTriggerOnOverlap)
    (bind _asbp_player (Utilities|Casting|CastToBP_Player OtherActor))
    (if (not (and (Variables|Default|GetbAutoTriggerOnlyOnce) (Variables|Default|GetbHasAutoTriggered)))
      (Variables|Default|SetbHasAutoTriggered true)
      (CallFunction|SpeaktoPlayer _asbp_player)
      (bind _wobble (Timeline|TL_TalkWobble PlayFromStart)
        (:Update
          (Transformation|SetWorldScale3D (Variables|Default|GetMesh) (Math|Vector|MakeVector _wobble _wobble _wobble)))))))

(event EventBeginPlay)

(event EventInteract
  (params (Sender :type Actor%20Object%20Reference))
  (bind _asbp_player (Utilities|Casting|CastToBP_Player Sender)
    (:then
      (CallFunction|SpeaktoPlayer _asbp_player)
      (bind _wobble (Timeline|TL_TalkWobble PlayFromStart)
        (:Update
          (Transformation|SetWorldScale3D (Variables|Default|GetMesh) (Math|Vector|MakeVector _wobble _wobble _wobble)))))
    (:CastFailed
      (Development|PrintString "PInteractSender im Hamster Event Graph schlägt fehl"))))

(fn ConstructionScript)

(fn GetNextDialogLine
  ;[0.15 0.15 0.15 0.5] Comment
  (if (> (Utilities|Array|Length (Variables|Default|GetDialogLines)) 0)
    (if (and (Variables|Default|GetbPlayOnlyOnce) (Variables|Default|GetbHasBeenUsed))
      _
      (else
        (Variables|Default|SetOutLine (Utilities|Array|Get(acopy) (Variables|Default|GetDialogLines) (Variables|Default|GetCurrentLineIndex)))
        (bind _output_get (Variables|Default|SetCurrentLineIndex (+ (Variables|Default|GetCurrentLineIndex) 1)))
        (if (>= _output_get (Utilities|Array|Length (Variables|Default|GetDialogLines)))
          (Variables|Default|SetbHasBeenUsed true)
          (Variables|Default|GetbLoopDialog
            (:then
              (Variables|Default|SetCurrentLineIndex 0))
            (:else
              (Variables|Default|SetCurrentLineIndex (- (Utilities|Array|Length (Variables|Default|GetDialogLines)) 1))))
          (return (Variables|Default|GetOutLine) true)
          (else
            (return (Variables|Default|GetOutLine) true))))))
  (return (Variables|Default|GetFallBackLine) true))

(fn SpeaktoPlayer
  (params (PlayerRef :type BP%20Player%20Object%20Reference))
  (bind (_outline _bhasvalidline) (CallFunction|GetNextDialogLine))
  (if _bhasvalidline
    (Transformation|SetActorRotation (Math|Rotator|FindLookatRotation (Transformation|GetActorLocation) (Transformation|GetActorLocation PlayerRef)))
    (Default|ShowTutorialDialog PlayerRef _outline)))

(fn ReturnInteractStatus
  (return (Variables|Default|GetIsInteractable)))