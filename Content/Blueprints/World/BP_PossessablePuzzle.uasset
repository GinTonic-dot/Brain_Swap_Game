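; Base possessable puzzle pawn that the player interacts with to take control.
; Interact raises the player's CanMove counter, saves control rotation, smooth-possesses the puzzle and pushes a widget onto the main stack.
; IA_Interact removes the widget, calls SmoothPosses again (also targeting self), restores rotation and lowers the counter.
; IA_Move resolves the dominant axis into empty Left, Right, Up and Down events, leaving puzzle logic unimplemented here.
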(event Custom|Down)

(event Custom|Left)

(event Custom|Right)

(event Custom|Up)

(event Input|EnhancedActionEvents|EnhancedInputActionIA_Interact
  (params (ActionValue :type Boolean) (ElapsedSeconds :type Float%20%28double-precision%29) (TriggeredSeconds :type Float%20%28double-precision%29) (InputAction :type Input%20Action%20Object%20Reference :default "/Game/Input/IA_Interact.IA_Interact"))
  (:Started
    (Utilities|FlowControl|DoOnce false :!label _label
      (:Completed
        (Class|CommonActivatableWidgetContainerBase|RemoveWidget (Utilities|ReturnMainStack (Game|GetPlayerController 0)) (Variables|Default|GetActiveWidget))
        (Utilities|SmoothPosses (Game|GetPlayerController 0) self 1.0)
        (Pawn|SetControlRotation (Game|GetPlayerController 0) (Variables|Default|GetControllRotation))
        (Math|Integer|DecrementInt (Variables|/Game/Blueprints/Core/BP_Player.BP_Player_C|GetCanMove (Variables|Default|GetPlayerRef))
          (:%20%20
            (goto _label Reset)))))))

(event Input|EnhancedActionEvents|EnhancedInputActionIA_Move
  (params (ActionValue :type Vector%202D%20Structure) (ElapsedSeconds :type Float%20%28double-precision%29) (TriggeredSeconds :type Float%20%28double-precision%29) (InputAction :type Input%20Action%20Object%20Reference :default "/Game/Input/IA_Move.IA_Move"))
  (bind (_x _y) (Math|Vector2D|BreakVector2D ActionValue))
  (:Started
    (if (> (Math|Float|Absolute(Float) _x) (Math|Float|Absolute(Float) _y))
      (if (> _x 0.0)
        (CallFunction|Right)
        (else
          (CallFunction|Left)))
      (elif (> _y 0.0)
        (CallFunction|Up)
        (else
          (CallFunction|Down))))))

(event EventInteract
  (params (Sender :type Actor%20Object%20Reference))
  (bind _asbp_player (Utilities|Casting|CastToBP_Player Sender))
  (bind _output_get (Variables|Default|SetPlayerRef _asbp_player))
  (Math|Integer|IncrementInt (Variables|/Game/Blueprints/Core/BP_Player.BP_Player_C|GetCanMove _output_get)
    (:%20%20
      (Variables|Default|SetControllRotation (Pawn|GetControlRotation (Variables|Default|GetPlayerRef) :!class /Script/Engine.Pawn))
      (Utilities|SmoothPosses (Game|GetPlayerController 0) self 1.0)
      (bind _returnvalue (Class|CommonActivatableWidgetContainerBase|AddWidget (Utilities|ReturnMainStack (Game|GetPlayerController 0)) (Variables|Default|GetActivatableWidget)))
      (Variables|Default|SetActiveWidget _returnvalue))))

(fn ConstructionScript)

(fn ReturnInteractStatus
  (return (Variables|Default|GetIsInteractable)))