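; BP_Lever is an interactable world lever that reports its ID to a LeverManager when pulled.
; BeginPlay caches the handle's starting rotation, and Interact, guarded by a check on IsPulled, snaps it to EndRotation and registers the input, printing a message if the manager is invalid.
; ResetLever clears the pulled flag and restores the starting rotation, while ReturnInteractStatus always returns true.
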(event EventBeginPlay
  (bind _output_get (Variables|Default|SetStartRotation (Variables|/Script/Engine.SceneComponent|GetRelativeRotation (Variables|Default|GetLeverHandle))))
  (Transformation|SetRelativeRotation (Variables|Default|GetLeverHandle) _output_get false false))

(event Collision|EventActorBeginOverlap
  (params (OtherActor :type Actor%20Object%20Reference)))

(event EventTick
  (params (DeltaSeconds :type Float%20%28single-precision%29)))

(event EventInteract
  (params (Sender :type Actor%20Object%20Reference))
  (Variables|Default|GetbIsPulled
    (:then)
    (:else
      (Variables|Default|SetbIsPulled true)
      (Transformation|SetRelativeRotation (Variables|Default|GetLeverHandle) (Variables|Default|GetEndRotation) false false)
      (bind _levermanager (Variables|Default|GetLeverManager)
        (:then
          (Default|RegisterLeverInput _levermanager (Variables|Default|GetLeverID)))
        (:else
          (Development|PrintString "LMRef not valid"))))))

(fn ConstructionScript)

(fn ResetLever
  (Variables|Default|SetbIsPulled false)
  (Transformation|SetRelativeRotation (Variables|Default|GetLeverHandle) (Variables|Default|GetStartRotation) false false))

(fn ReturnInteractStatus
  (return true))