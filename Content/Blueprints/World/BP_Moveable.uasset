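; BP_Moveable is an interactable world object, such as a door, that eases a scene component between its start and target transforms.
; Interact can require the player's held collectable to match an ID and optionally consumes it, while non-player senders and React bypass that check.
; A FlipFlop alternates the destination as a door animation plays, then the MoveOnce check either re-enables interaction or also destroys the actor.
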(event EventBeginPlay
  (Variables|Default|SetStartTransform (Transformation|GetRelativeTransform (Variables|Default|GetMoveScene))))

(event EventReact
  (params (Solved :type Boolean))
  (bind _isa (Utilities|FlowControl|FlipFlop)
    (:A
      _)
    (:B
      _))
  (Components|Animation|PlayAnimation (Variables|Default|GetAnimatedMesh) "/Game/FBX/TürmitTürSkeletal_Anim.TürmitTürSkeletal_Anim" false)
  (Components|MoveComponentTo (Variables|Default|GetMoveScene) (.Location (Math|Transform|BreakTransform (Math|Transform|SelectTransform (Variables|Default|GetTargetTransform) (Variables|Default|GetStartTransform) _isa))) (.Rotation (Math|Transform|BreakTransform (Math|Transform|SelectTransform (Variables|Default|GetTargetTransform) (Variables|Default|GetStartTransform) _isa))) true true (Variables|Default|GetMoveDuration) true)
  (Variables|Default|GetMoveOnce
    (:then
      (Variables|Default|SetIsInteractable true))
    (:else
      (Variables|Default|SetIsInteractable true)
      (Actor|DestroyActor self))))

(event EventInteract
  (params (Sender :type Actor%20Object%20Reference))
  (Class|KismetSystemLibrary|IsObjectOfSoftClass Sender "/Game/Blueprints/Core/BP_Player.BP_Player_C"
    (:True
      ;[1 1 1] Check for ID
      (bind _asbp_player (Utilities|Casting|CastToBP_Player Sender))
      (if (Utilities|Array|IsEmpty (Variables|Default|GetNeededID))
        (Variables|Default|SetIsInteractable false :!label _label)
        (bind _isa (Utilities|FlowControl|FlipFlop)
          (:A
            _)
          (:B
            _))
        (Components|Animation|PlayAnimation (Variables|Default|GetAnimatedMesh) "/Game/FBX/TürmitTürSkeletal_Anim.TürmitTürSkeletal_Anim" false)
        (Components|MoveComponentTo (Variables|Default|GetMoveScene) (.Location (Math|Transform|BreakTransform (Math|Transform|SelectTransform (Variables|Default|GetTargetTransform) (Variables|Default|GetStartTransform) _isa))) (.Rotation (Math|Transform|BreakTransform (Math|Transform|SelectTransform (Variables|Default|GetTargetTransform) (Variables|Default|GetStartTransform) _isa))) true true (Variables|Default|GetMoveDuration) true)
        (Variables|Default|GetMoveOnce
          (:then
            (Variables|Default|SetIsInteractable true))
          (:else
            (Variables|Default|SetIsInteractable true)
            (Actor|DestroyActor self)))
        (else
          (Utilities|IsValid (Variables|/Game/Blueprints/Core/BP_Player.BP_Player_C|GetHeldCollectable _asbp_player)
            (:Is%20Valid
              (if (Utilities|Enum|Equal(Enum) (Variables|/Game/Blueprints/World/BP_Collectable.BP_Collectable_C|GetID (Variables|/Game/Blueprints/Core/BP_Player.BP_Player_C|GetHeldCollectable _asbp_player)) (Variables|Default|GetNeededID))
                (Variables|Default|GetDestroyItem
                  (:then
                    (Variables|Default|SetNeededID "")
                    (Actor|DestroyActor (Variables|/Game/Blueprints/Core/BP_Player.BP_Player_C|GetHeldCollectable _asbp_player))
                    (Variables|/Game/Blueprints/Core/BP_Player.BP_Player_C|SetHeldCollectable _asbp_player 0)
                    (goto _label))
                  (:else
                    (goto _label)))))
            (:Is%20Not%20Valid)))))
    (:False
      (goto _label))))

(fn ConstructionScript)

(fn ReturnInteractStatus
  (return (Variables|Default|GetIsInteractable)))