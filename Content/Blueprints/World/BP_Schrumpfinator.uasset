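; BP_Schrumpfinator is an interactable world actor that toggles the player between shrunken and normal size.
; On Interact, a FlipFlop alternates between resizing the player's capsule down and restoring it, adjusting camera FOV and look sensitivity to match.
; Restoring also nudges the player upward to offset the larger capsule.
; The shrink state lives only in this actor's FlipFlop, and ReturnInteractStatus always returns true.
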(event EventInteract
  (params (Sender :type Actor%20Object%20Reference))
  (bind _returnvalue (Game|GetPlayerCharacter 0))
  (bind _capsulecomponent (Variables|/Script/Engine.Character|GetCapsuleComponent _returnvalue))
  (bind _asbp_player (Utilities|Casting|CastToBP_Player _returnvalue))
  (Utilities|FlowControl|FlipFlop
    (:A
      (Components|Capsule|SetCapsuleSize _capsulecomponent 6.0 1e+01 true)
      (Development|PrintString "Is Shrinked True")
      (Camera|SetFieldOfView (Variables|/Game/Blueprints/Core/BP_Player.BP_Player_C|GetCamera _asbp_player) 7e+01)
      (Variables|/Game/Blueprints/Core/BP_Player.BP_Player_C|SetLookSens _asbp_player 0.4))
    (:B
      (Components|Capsule|SetCapsuleSize _capsulecomponent 34.0 88.0 false)
      (Transformation|AddActorWorldOffset _returnvalue (Math|Vector|MakeVector 0.0 0.0 4e+01))
      (Development|PrintString "Is Shrinked False")
      (Camera|SetFieldOfView (Variables|/Game/Blueprints/Core/BP_Player.BP_Player_C|GetCamera _asbp_player) 9e+01)
      (Variables|/Game/Blueprints/Core/BP_Player.BP_Player_C|SetLookSens _asbp_player 1.5))))

(fn ConstructionScript)

(fn ReturnInteractStatus
  (return true))