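; BP_CodeManager runs a lever-sequence puzzle, tracking progress toward a correct order of lever IDs.
; RegisterLeverInput compares each pulled lever ID with the next expected one, advancing on a match or resetting progress and all connected levers on a mistake.
; Completing the sequence sets Solved, sends ReactMessage to the actors in ActorToReact and plays a sound.
; Solved blocks further input and is exposed through ReturnSolvedStatus; PuzzleComplete is empty.
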(event EventBeginPlay)

(event Collision|EventActorBeginOverlap
  (params (OtherActor :type Actor%20Object%20Reference)))

(event EventTick
  (params (DeltaSeconds :type Float%20%28single-precision%29)))

(fn ConstructionScript)

(fn RegisterLeverInput
  (params (PulledLeverID :type Integer))
  (Development|PrintString "RegisterLeverInput")
  (if (not (Variables|Default|GetSolved))
    (if (< (Variables|Default|GetCurrentIndex) (Utilities|Array|Length (Variables|Default|GetCorrectSequence)))
      (if (== PulledLeverID (Utilities|Array|Get(acopy) (Variables|Default|GetCorrectSequence) (Variables|Default|GetCurrentIndex)))
        (bind _output_get (Variables|Default|SetCurrentIndex (+ (Variables|Default|GetCurrentIndex) 1)))
        (if (>= _output_get (Utilities|Array|Length (Variables|Default|GetCorrectSequence)))
          (Variables|Default|SetSolved true)
          (for _array_element (Variables|Default|GetActorToReact)
            (Class|BPIReact|React(Message) _array_element true)
            (Development|PrintString "Solved Lever")
            (Audio|PlaySound2D 0 1.0 1.0 0.0 0 0)))
        (else
          (CallFunction|ResetPuzzle)
          (Development|PrintString "Reset Lever")
          (Audio|PlaySound2D 0 1.0 1.0 0.0 0 0))))))

(fn ResetPuzzle
  (Variables|Default|SetCurrentIndex 0)
  (for _array_element (Variables|Default|GetConnectedLevers)
    (Default|ResetLever _array_element)))

(fn PuzzleComplete)

(fn ReturnSolvedStatus
  (return (Variables|Default|GetSolved)))