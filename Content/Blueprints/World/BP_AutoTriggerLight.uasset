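; BP_AutoTriggerLight is a world light that switches on automatically, along with a Niagara effect, while something overlaps its trigger volume.
; It starts hidden with the effect inactive.
; Overlap begin shows the spotlight, animates its intensity with the LichtIntensität timeline and activates Niagara.
; Overlap end deactivates Niagara and plays a separate timeline in reverse from its end, hiding the light when finished, with no filtering on the overlapping actor.
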(event OnComponentBeginOverlap(TriggerCollision)
  (params (OverlappedComponent :type Primitive%20Component%20Object%20Reference) (OtherActor :type Actor%20Object%20Reference) (OtherComp :type Primitive%20Component%20Object%20Reference) (OtherBodyIndex :type Integer) (bFromSweep :type Boolean) (SweepResult :type Hit%20Result%20Structure%20%28by%20ref%29))
  (bind _spotlight (Variables|Default|GetSpotLight))
  (Utilities|FlowControl|Sequence
    (:then_0
      (Rendering|SetVisibility _spotlight true false)
      (bind _intensität (Timeline|LichtIntensität PlayFromStart)
        (:Update
          (Rendering|Components|Light|SetIntensity _spotlight _intensität))))
    (:then_1
      (Components|Activation|Activate (Variables|Default|GetNiagara) false))))

(event OnComponentEndOverlap(TriggerCollision)
  (params (OverlappedComponent :type Primitive%20Component%20Object%20Reference) (OtherActor :type Actor%20Object%20Reference) (OtherComp :type Primitive%20Component%20Object%20Reference) (OtherBodyIndex :type Integer))
  (Utilities|FlowControl|Sequence
    (:then_0
      (bind _intensität (Timeline|Timeline ReverseFromEnd)
        (:Update
          (Rendering|Components|Light|SetIntensity (Variables|Default|GetSpotLight) _intensität))
        (:Finished
          (Rendering|SetVisibility (Variables|Default|GetSpotLight) false false))))
    (:then_1
      (Components|Activation|Deactivate (Variables|Default|GetNiagara)))))

(event EventBeginPlay
  (bind _spotlight (Variables|Default|GetSpotLight))
  (Components|Activation|Deactivate (Variables|Default|GetNiagara))
  (Rendering|SetVisibility _spotlight false false)
  (Rendering|Components|Light|SetIntensity _spotlight 1e+03))

(fn ConstructionScript)