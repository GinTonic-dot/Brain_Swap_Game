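; Moving-object actor that carries a list of actors along its spline, spaced by a fixed distance offset.
; A timeline, with rate set from PlayRate, drives distance along the spline, wrapping each actor once past the end.
; Actors take the world spline location but use a Rotation variable instead of spline rotation.
; With Loop set, the timeline replays from the start; its Reverse call is immediately overridden by PlayFromStart.
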(event Custom|PlayTimelineReverse
  (bind _spline (Variables|Default|GetSpline))
  (bind _returnvalue (Spline|GetSplineLength _spline))
  (bind (_direction _alpha) (Timeline|Timeline Reverse)
    (:Update
      (for (_array_element _array_index) (Variables|Default|GetActors)
        (bind _output_get (Variables|Default|SetDistanceAlongSpline (+ (Math|Float|Lerp 0.0 (Spline|GetSplineLength (Variables|Default|GetSpline)) _alpha) (* _array_index (Variables|Default|GetOffsetBetweenActors)))))
        (if (> _output_get _returnvalue)
          (Variables|Default|SetDistanceAlongSpline (- (Variables|Default|GetDistanceAlongSpline) _returnvalue)))
        (Transformation|SetActorLocationAndRotation _array_element (Spline|GetLocationatDistanceAlongSpline (Variables|Default|GetSpline) (Variables|Default|GetDistanceAlongSpline) "World") (Variables|Default|GetRotation) false (Variables|Default|GetbTeleport))))
    (:Finished
      (if (Variables|Default|GetbLoop)
        (switch Utilities|FlowControl|Switch|SwitchonETimelineDirection _direction
          (:Forward
            (CallFunction|PlayTimelineReverse)
            (CallFunction|DetailsPlayTimeline))
          (:Backward
            (CallFunction|DetailsPlayTimeline)))))))

(event Custom|DetailsPlayTimeline
  (bind _spline (Variables|Default|GetSpline))
  (bind _returnvalue (Spline|GetSplineLength _spline))
  (bind (_direction _alpha) (Timeline|Timeline PlayFromStart)
    (:Update
      (for (_array_element _array_index) (Variables|Default|GetActors)
        (bind _output_get (Variables|Default|SetDistanceAlongSpline (+ (Math|Float|Lerp 0.0 (Spline|GetSplineLength (Variables|Default|GetSpline)) _alpha) (* _array_index (Variables|Default|GetOffsetBetweenActors)))))
        (if (> _output_get _returnvalue)
          (Variables|Default|SetDistanceAlongSpline (- (Variables|Default|GetDistanceAlongSpline) _returnvalue)))
        (Transformation|SetActorLocationAndRotation _array_element (Spline|GetLocationatDistanceAlongSpline (Variables|Default|GetSpline) (Variables|Default|GetDistanceAlongSpline) "World") (Variables|Default|GetRotation) false (Variables|Default|GetbTeleport))))
    (:Finished
      (if (Variables|Default|GetbLoop)
        (switch Utilities|FlowControl|Switch|SwitchonETimelineDirection _direction
          (:Forward
            (CallFunction|PlayTimelineReverse)
            (CallFunction|DetailsPlayTimeline))
          (:Backward
            (CallFunction|DetailsPlayTimeline)))))))

(event EventBeginPlay
  (Components|Timeline|SetPlayRate (Variables|Default|GetTimeline) (/ 1.0 (Variables|Default|GetPlay%20Rate)))
  (CallFunction|DetailsPlayTimeline))

(fn ConstructionScript)