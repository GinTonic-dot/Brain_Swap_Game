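; Test puzzle socket that holds one collectable and signals ActorToReact when the item with the needed ID is placed.
; Interact lets the player take the socketed item when empty-handed, or snap their held item into an empty socket.
; A collected-dispatcher binding clears the socket on pickup and revokes the solved state.
; A preassigned collectable snaps into place in the construction script and at BeginPlay.
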(event Custom|OnCurrentCollectablePickedUp
  (bind _currentcollactable (Variables|Default|GetCurrentCollactable)
    (:then
      (EventDispatchers|UnbindEventfromOnCollectedDispatcher _currentcollactable (delegate Custom|OnCurrentCollectablePickedUp))
      (Variables|Default|SetCurrentCollactable 0)
      (Variables|Default|GetSolved
        (:then
          (Variables|Default|SetSolved false)
          (Class|BPIReact|React(Message) (Variables|Default|GetActorToReact) false))
        (:else)))
    (:else)))

(event EventBeginPlay
  (bind _currentcollactable (Variables|Default|GetCurrentCollactable)
    (:then
      (Transformation|AttachComponentToComponent _currentcollactable (Variables|Default|GetCollectableScene) "None" "SnapToTarget" "SnapToTarget" "SnapToTarget" true)
      (EventDispatchers|BindEventtoOnCollectedDispatcher (Variables|Default|GetCurrentCollactable) (EventDispatchers|CreateEvent :!event Custom|OnCurrentCollectablePickedUp)))
    (:else)))

(event EventInteract
  (params (Sender :type Actor%20Object%20Reference))
  (Class|KismetSystemLibrary|IsObjectOfSoftClass Sender "/Game/Blueprints/Core/BP_Player.BP_Player_C"
    (:True
      (Variables|Default|GetPlayerRef
        (:then
          _)
        (:else
          (bind _asbp_player (Utilities|Casting|CastToBP_Player Sender))
          (Variables|Default|SetPlayerRef _asbp_player)))
      (Variables|Default|GetCurrentCollactable
        (:then
          (Variables|/Game/Blueprints/Core/BP_Player.BP_Player_C|GetHeldCollectable (Variables|Default|GetPlayerRef)
            (:then)
            (:else
              (Class|BPIInteract|Interact(Message) (Variables|Default|GetCurrentCollactable) (Variables|Default|GetPlayerRef)))))
        (:else
          (bind _heldcollectable (Variables|/Game/Blueprints/Core/BP_Player.BP_Player_C|GetHeldCollectable (Variables|Default|GetPlayerRef))
            (:then
              (Transformation|AttachComponentToComponent _heldcollectable (Variables|Default|GetCollectableScene) "None" "SnapToTarget" "SnapToTarget" "SnapToTarget" true)
              (Default|PlaceCollectable _heldcollectable)
              (bind _output_get (Variables|Default|SetCurrentCollactable _heldcollectable))
              (EventDispatchers|BindEventtoOnCollectedDispatcher _output_get (EventDispatchers|CreateEvent :!event Custom|OnCurrentCollectablePickedUp))
              (Variables|/Game/Blueprints/Core/BP_Player.BP_Player_C|SetHeldCollectable (Variables|Default|GetPlayerRef) 0)
              (if (Utilities|Enum|Equal(Enum) (Variables|/Game/Blueprints/World/BP_Collectable.BP_Collectable_C|GetID (Variables|Default|GetCurrentCollactable)) (Variables|Default|GetNeededID))
                (Variables|Default|SetSolved true)
                (Class|BPIReact|React(Message) (Variables|Default|GetActorToReact) true)))
            (:else)))))))

(event EventSetInteractStatus
  (params (IsInteractable :type Boolean))
  (Variables|Default|SetIsInteractable IsInteractable)
  (Class|BPIInteract|SetInteractStatus(Message) (Variables|Default|GetCurrentCollactable) IsInteractable))

(fn ConstructionScript
  (bind _currentcollactable (Variables|Default|GetCurrentCollactable)
    (:then
      (Transformation|AttachComponentToComponent _currentcollactable (Variables|Default|GetCollectableScene) "None" "SnapToTarget" "SnapToTarget" "SnapToTarget" true))
    (:else)))

(fn ReturnInteractStatus
  (return (Variables|Default|GetIsInteractable)))

(fn ReturnSolvedStatus
  (return (Variables|Default|GetSolved)))