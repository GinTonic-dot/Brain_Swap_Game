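; BP_SnapSocket is a test-folder snap socket Blueprint that appears meant to gate which blocks can occupy it.
; CanAcceptBlock checks allowed shape and yaw-index lists against fixed placeholder values instead of the Block's properties, consulting Occupied only when the Block is invalid.
; SetOccupied ignores its Block input and always clears the occupancy flag and occupying block.
; Events and construction script are empty, so the logic looks unfinished.
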(event EventBeginPlay)

(event Collision|EventActorBeginOverlap
  (params (OtherActor :type Actor%20Object%20Reference)))

(event EventTick
  (params (DeltaSeconds :type Float%20%28single-precision%29)))

(fn ConstructionScript)

(fn CanAcceptBlock
  (params (Block :type BP%20Tetris%20Block%20Object%20Reference))
  (Utilities|IsValid Block
    (:Is%20Valid
      (bind _output_get (Variables|Default|SetbShapeOK (Utilities|Array|ContainsItem (Variables|Default|GetAllowedShapes) "NewEnumerator0")))
      (bind _output_get_2 (Variables|Default|SetbRotOK (Utilities|Array|ContainsItem (Variables|Default|GetAllowedYawIndices) 0)))
      (return (and _output_get _output_get_2)))
    (:Is%20Not%20Valid
      (if (Variables|Default|GetbOccupied)
        (return (and _output_get _output_get_2))))))

(fn SetOccupied
  (params (Block :type BP%20Tetris%20Block%20Object%20Reference))
  (bind _output_get (Variables|Default|SetbOccupied false))
  (Variables|Default|SetOccupyingBlock 0)
  (return _output_get 0))